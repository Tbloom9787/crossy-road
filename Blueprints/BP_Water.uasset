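; Lane tile for a Crossy Road-style chicken game that, despite its name, can become grass, road, water or train track.
; RandomizeMesh rolls the type with odds that shift as the chicken's TileCounter grows, then has Spawner add matching props, coins and hazards.
; Counters on the chicken drive alternating grass shades, road lines and lily pad spacing.
; Chicken overlap with TriggerZone calls SpawnWaterAtSpawnPoint, destroys the tile and assigns it to the chicken's Water reference.
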(event OnComponentBeginOverlap(TriggerZone)
  (params (OverlappedComponent :type Primitive%20Component%20Object%20Reference) (OtherActor :type Actor%20Object%20Reference) (OtherComp :type Primitive%20Component%20Object%20Reference) (OtherBodyIndex :type Integer) (bFromSweep :type Boolean) (SweepResult :type Hit%20Result%20Structure%20%28by%20ref%29))
  (bind _asbpc_chicken (Utilities|Casting|CastToBPC_Chicken OtherActor))
  (Default|SpawnWateratSpawnPoint (Variables|Default|GetSpawner))
  (Actor|DestroyActor)
  (Variables|/Game/Blueprints/BPC_Chicken.BPC_Chicken_C|SetWater _asbpc_chicken self))

(event EventBeginPlay)

(event Collision|EventActorBeginOverlap
  (params (OtherActor :type Actor%20Object%20Reference)))

(event EventTick
  (params (DeltaSeconds :type Float%20%28single-precision%29)))

(fn ConstructionScript)

(fn RandomizeMesh
  (bind _returnvalue (Math|Random|RandomIntegerinRange 0 2))
  (bind _outactors (Actor|GetAllActorsOfClass "/Game/Blueprints/BPC_Chicken.BPC_Chicken_C"))
  (Variables|Default|SetChicken (Utilities|Array|Get(acopy) _outactors))
  (if (> (Variables|/Game/Blueprints/BPC_Chicken.BPC_Chicken_C|GetTileCounter (Variables|Default|GetChicken)) 100)
    (if (> (Variables|/Game/Blueprints/BPC_Chicken.BPC_Chicken_C|GetTileCounter (Variables|Default|GetChicken)) 200)
      (switch int (Math|Random|RandomIntegerinRange 0 10)
        (:0
          (Components|StaticMesh|SetStaticMesh (Variables|Default|GetStaticMesh) "/Game/Characters/Grass/grass.grass" :!label _label)
          (bind _asbpc_chicken (Utilities|Casting|CastToBPC_Chicken (Game|GetPlayerCharacter 0)))
          (Variables|/Game/Blueprints/BPC_Chicken.BPC_Chicken_C|Setroadcount _asbpc_chicken 0)
          (bind _asbpc_chicken_2 (Utilities|Casting|CastToBPC_Chicken (Game|GetPlayerCharacter 0)))
          (bind _output_get (Variables|/Game/Blueprints/BPC_Chicken.BPC_Chicken_C|Setgrasscounter _asbpc_chicken_2 (+ (Variables|/Game/Blueprints/BPC_Chicken.BPC_Chicken_C|Getgrasscounter _asbpc_chicken_2) 1)))
          (if (== (Math|Integer|%(Integer) _output_get 2) 0)
            (Components|StaticMesh|SetStaticMesh (Variables|Default|GetStaticMesh) "/Game/Characters/Grass/DarkGrass.DarkGrass"))
          (bind _asbpc_chicken_3 (Utilities|Casting|CastToBPC_Chicken (Game|GetPlayerCharacter 0)))
          (Variables|/Game/Blueprints/BPC_Chicken.BPC_Chicken_C|Setlily _asbpc_chicken_3 false)
          (Default|SpawnCoin (Variables|Default|GetSpawner) (Transformation|GetWorldLocation (Variables|Default|GetSpawnPoint)))
          (if (== _returnvalue 0)
            (Default|SpawnSmallBush (Variables|Default|GetSpawner) (Transformation|GetWorldLocation (Variables|Default|GetSpawnPoint)))
            (elif (== _returnvalue 1)
              (Default|SpawnTree (Variables|Default|GetSpawner) (Transformation|GetWorldLocation (Variables|Default|GetSpawnPoint)))
              (else
                (Default|SpawnRock (Variables|Default|GetSpawner) (Transformation|GetWorldLocation (Variables|Default|GetSpawnPoint)))))))
        (:1
          (Components|StaticMesh|SetStaticMesh (Variables|Default|GetStaticMesh) "/Game/Characters/Road/road.road" :!label _label_2)
          (bind _asbpc_chicken_4 (Utilities|Casting|CastToBPC_Chicken (Game|GetPlayerCharacter 0)))
          (Variables|Default|SetIsRoad true)
          (Variables|/Game/Blueprints/BPC_Chicken.BPC_Chicken_C|Setroadcount _asbpc_chicken_4 (+ (Variables|/Game/Blueprints/BPC_Chicken.BPC_Chicken_C|Getroadcount _asbpc_chicken_4) 1))
          (bind _asbpc_chicken_5 (Utilities|Casting|CastToBPC_Chicken (Game|GetPlayerCharacter 0)))
          (Variables|/Game/Blueprints/BPC_Chicken.BPC_Chicken_C|Setlily _asbpc_chicken_5 false)
          (Default|SpawnCoin (Variables|Default|GetSpawner) (Transformation|GetWorldLocation (Variables|Default|GetSpawnPoint)))
          (if (== (Math|Random|RandomIntegerinRange 0 1) 0)
            (Default|SpawnCar (Variables|Default|GetSpawner) (Transformation|GetWorldLocation (Variables|Default|GetSpawnPoint)))
            (bind _asbpc_chicken_6 (Utilities|Casting|CastToBPC_Chicken (Game|GetPlayerCharacter 0)))
            (if (> (Variables|/Game/Blueprints/BPC_Chicken.BPC_Chicken_C|Getroadcount _asbpc_chicken_6) 1)
              (Default|SpawnRoadLines (Variables|Default|GetSpawner) (Transformation|GetWorldLocation (Variables|Default|GetSpawnPoint))))
            (else
              (Default|SpawnTruck (Variables|Default|GetSpawner) (Transformation|GetWorldLocation (Variables|Default|GetSpawnPoint)))
              (bind _asbpc_chicken_7 (Utilities|Casting|CastToBPC_Chicken (Game|GetPlayerCharacter 0)))
              (if (> (Variables|/Game/Blueprints/BPC_Chicken.BPC_Chicken_C|Getroadcount _asbpc_chicken_7) 1)
                (Default|SpawnRoadLines (Variables|Default|GetSpawner) (Transformation|GetWorldLocation (Variables|Default|GetSpawnPoint)))))))
        (:2
          (goto _label_2))
        (:3
          (goto _label_2))
        (:4
          (goto _label_2))
        (:5
          (goto _label_2))
        (:6
          (Components|StaticMesh|SetStaticMesh (Variables|Default|GetStaticMesh) "/Game/Characters/Water/water.water" :!label _label_3)
          (bind _asbpc_chicken_8 (Utilities|Casting|CastToBPC_Chicken (Game|GetPlayerCharacter 0)))
          (Variables|/Game/Blueprints/BPC_Chicken.BPC_Chicken_C|Setroadcount _asbpc_chicken_8 0)
          (Variables|Default|SetIsWater true)
          (if (== (Math|Random|RandomIntegerinRange 0 3) 0)
            (bind _asbpc_chicken_9 (Utilities|Casting|CastToBPC_Chicken (Game|GetPlayerCharacter 0)))
            (if (Variables|/Game/Blueprints/BPC_Chicken.BPC_Chicken_C|Getlily _asbpc_chicken_9)
              (if (== (Math|Random|RandomIntegerinRange 0 1) 0) :!label _label_4
                (Default|SpawnLog (Variables|Default|GetSpawner) (Transformation|GetWorldLocation (Variables|Default|GetSpawnPoint)))
                (else
                  (Default|SpawnLongLog (Variables|Default|GetSpawner) (Transformation|GetWorldLocation (Variables|Default|GetSpawnPoint)))))
              (else
                (Default|SpawnLilyPad (Variables|Default|GetSpawner) (Transformation|GetWorldLocation (Variables|Default|GetSpawnPoint)))
                (bind _asbpc_chicken_10 (Utilities|Casting|CastToBPC_Chicken (Game|GetPlayerCharacter 0)))
                (Variables|/Game/Blueprints/BPC_Chicken.BPC_Chicken_C|Setlily _asbpc_chicken_10 true)))
            (else
              (goto _label_4))))
        (:7
          (Components|StaticMesh|SetStaticMesh (Variables|Default|GetStaticMesh) "/Game/Characters/Road/road.road" :!label _label_5)
          (bind _asbpc_chicken_11 (Utilities|Casting|CastToBPC_Chicken (Game|GetPlayerCharacter 0)))
          (Variables|/Game/Blueprints/BPC_Chicken.BPC_Chicken_C|Setroadcount _asbpc_chicken_11 0)
          (bind _asbpc_chicken_12 (Utilities|Casting|CastToBPC_Chicken (Game|GetPlayerCharacter 0)))
          (Variables|/Game/Blueprints/BPC_Chicken.BPC_Chicken_C|Setlily _asbpc_chicken_12 false)
          (Default|SpawnCoin (Variables|Default|GetSpawner) (Transformation|GetWorldLocation (Variables|Default|GetSpawnPoint)))
          (Default|SpawnTrainTracks (Variables|Default|GetSpawner) (Transformation|GetWorldLocation (Variables|Default|GetSpawnPoint)))
          (Default|SpawnTrainPost (Variables|Default|GetSpawner) (Transformation|GetWorldLocation (Variables|Default|GetSpawnPoint)))
          (Default|SpawnTrain (Variables|Default|GetSpawner) (Transformation|GetWorldLocation (Variables|Default|GetSpawnPoint))))
        (:8
          (goto _label_5))
        (:9
          (goto _label_5))
        (:10
          (goto _label_5)))
      (else
        (switch int (Math|Random|RandomIntegerinRange 0 10)
          (:0
            (goto _label))
          (:1
            (goto _label_2))
          (:2
            (goto _label_2))
          (:3
            (goto _label_2))
          (:4
            (goto _label_2))
          (:5
            (goto _label_3))
          (:6
            (goto _label_3))
          (:7
            (goto _label_5))
          (:8
            (goto _label_5))
          (:9
            (goto _label_3))
          (:10
            (goto _label)))))
    (else
      (switch int (Math|Random|RandomIntegerinRange 0 3)
        (:0
          (goto _label))
        (:1
          (goto _label_2))
        (:2
          (goto _label_3))
        (:3
          (goto _label_5))))))

(fn InitialGrass
  (Components|StaticMesh|SetStaticMesh (Variables|Default|GetStaticMesh) "/Game/Characters/Grass/grass.grass"))