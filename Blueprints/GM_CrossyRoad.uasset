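; Game mode for a Crossy Road-style game that caches references to the chicken and the HUD.
; BeginPlay takes the first BPC_Chicken actor and top-level WBP_HUD widget, and sets the chicken's GMCrossy reference to None rather than to itself.
; Logic that copies the chicken's Highscore and refreshes the HUD is disconnected and never runs.
; Tick and the construction script are empty.
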(event EventBeginPlay
  (bind _outactors (Actor|GetAllActorsOfClass "/Game/Blueprints/BPC_Chicken.BPC_Chicken_C"))
  (Variables|/Game/Blueprints/BPC_Chicken.BPC_Chicken_C|SetGM_Crossy (Utilities|Array|Get(acopy) _outactors) 0)
  (Variables|Default|Setchicken (Utilities|Array|Get(acopy) _outactors))
  (bind _foundwidgets (Widget|GetAllWidgetsOfClass "/Game/UI/WBP_HUD.WBP_HUD_C" true))
  (Variables|Default|SetHUD (Utilities|Array|Get(acopy) _foundwidgets)))

(event EventTick
  (params (DeltaSeconds :type Float%20%28single-precision%29)))

(fn ConstructionScript)