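; BP_Chicken is a player-controlled chicken pawn with simple directional movement.
; MoveForward and MoveRight axes add input along actor vectors scaled by MaxSpeed, which Tick consumes as a frame-time-scaled local offset without sweeping.
; W, A, S and D presses snap only the static mesh's yaw to the matching direction.
; RFront stores the starting rotation but feeds only an unconnected comparison.
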(event EventBeginPlay
  (Variables|Default|SetR_Front (Transformation|GetActorRotation)))

(event Collision|EventActorBeginOverlap
  (params (OtherActor :type Actor%20Object%20Reference)))

(event EventTick
  (params (DeltaSeconds :type Float%20%28single-precision%29))
  (bind _returnvalue (Class|Pawn|ConsumeMovementInputVector))
  (Transformation|AddActorLocalOffset (* _returnvalue DeltaSeconds) false false))

(event Input|ActionEvents|InputActionMoveForward
  (params (Key :type Key%20Structure)))

(event Input|AxisEvents|InputAxisMoveForward
  (params (AxisValue :type Float%20%28single-precision%29))
  (Pawn|Input|AddMovementInput (Transformation|GetActorForwardVector) (* AxisValue (Variables|Default|GetMaxSpeed)) false))

(event Input|AxisEvents|InputAxisMoveRight
  (params (AxisValue :type Float%20%28single-precision%29))
  (Pawn|Input|AddMovementInput (Transformation|GetActorRightVector) (* AxisValue (Variables|Default|GetMaxSpeed)) false))

(event Input|KeyboardEvents|A
  (params (Key :type Key%20Structure))
  (:Pressed
    (Transformation|SetRelativeRotation (Variables|Default|GetStaticMesh) "0,-90.000000, 0" false false)))

(event Input|KeyboardEvents|W
  (params (Key :type Key%20Structure))
  (:Pressed
    (Transformation|SetRelativeRotation (Variables|Default|GetStaticMesh) "0, 0, 0" false false)))

(event Input|KeyboardEvents|D
  (params (Key :type Key%20Structure))
  (:Pressed
    (Transformation|SetRelativeRotation (Variables|Default|GetStaticMesh) "0,90.000000,0.000000" false false)))

(event Input|KeyboardEvents|S
  (params (Key :type Key%20Structure))
  (:Pressed
    (Transformation|SetRelativeRotation (Variables|Default|GetStaticMesh) "0,180.000000,0.000000" false false)))

(fn ConstructionScript)