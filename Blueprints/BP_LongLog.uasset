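; BP_LongLog is a log actor that drifts continuously along the negative Y axis and loops back when it passes a limit.
; BeginPlay picks a random speed, and Tick applies a world offset scaled by delta time.
; Once the log passes a fixed Y threshold, Tick shifts it forward by a fixed distance, so the same actor is reused in an endless loop.
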(event EventBeginPlay
  (Variables|Default|Setmax_speed (Math|Random|RandomFloatinRange 1e+02 2e+02)))

(event Collision|EventActorBeginOverlap
  (params (OtherActor :type Actor%20Object%20Reference)))

(event EventTick
  (params (DeltaSeconds :type Float%20%28single-precision%29))
  (bind _returnvalue (Transformation|GetActorLocation))
  (Transformation|AddActorWorldOffset (Math|Vector|MakeVector 0.0 (* (* DeltaSeconds (Variables|Default|Getmax_speed)) -1.0) 0.0))
  (if (< (.y (Transformation|GetActorLocation)) -1.3e+03)
    (Transformation|SetActorLocation (Math|Vector|MakeVector (.x _returnvalue) (+ (.y _returnvalue) 2e+03) (.z _returnvalue)) false false)))

(fn ConstructionScript)